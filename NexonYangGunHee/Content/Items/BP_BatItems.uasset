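; BP_BatItems is an item actor that notifies the player when they are within its interaction range.
; InteractionBox switches to query-only collision shortly after BeginPlay, and its overlap events call StartTraceMessage on the player character to start or stop tracing for this item.
; The construction script applies ItemTransform to PosStoreComp as its relative transform.
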(event OnComponentBeginOverlap(InteractionBox)
  (params (OverlappedComponent :type Primitive%20Component%20Object%20Reference) (OtherActor :type Actor%20Object%20Reference) (OtherComp :type Primitive%20Component%20Object%20Reference) (OtherBodyIndex :type Integer) (bFromSweep :type Boolean) (SweepResult :type Hit%20Result%20Structure%20%28by%20ref%29))
  (bind _returnvalue (Game|GetPlayerCharacter 0))
  (if (== OtherActor _returnvalue)
    (Class|BPCharacterInterface|StartTrace(Message) _returnvalue false self)))

(event OnComponentEndOverlap(InteractionBox)
  (params (OverlappedComponent :type Primitive%20Component%20Object%20Reference) (OtherActor :type Actor%20Object%20Reference) (OtherComp :type Primitive%20Component%20Object%20Reference) (OtherBodyIndex :type Integer))
  (bind _returnvalue (Game|GetPlayerCharacter 0))
  (if (== OtherActor _returnvalue)
    (Class|BPCharacterInterface|StartTrace(Message) _returnvalue true self)))

(event EventBeginPlay
  (Utilities|FlowControl|Delay 0.2)
  (Collision|SetCollisionEnabled (Variables|Default|GetInteraction%20Box) "QueryOnly"))

(fn ConstructionScript
  (Transformation|SetRelativeTransform (Variables|Default|GetPosStoreComp) (Variables|Default|GetItemTransform) false false))