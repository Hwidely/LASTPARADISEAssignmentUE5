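; Zombie girl enemy character that can be fought or stealth-killed by the third-person player.
; A box overlap offers the player an assassination prompt while the zombie is undetected.
; Capsule overlaps handle weapon, block and BP_BatShoot hits, triggering AI detection and animation flags, with player attacks using weapon row data for damage, effects and knockdown.
; Tick turns the HP text toward the camera and triggers delayed-destroy death at zero HP; a timer loops zombie sounds.
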(event OnComponentBeginOverlap(CapsuleComponent)
  (params (OverlappedComponent :type Primitive%20Component%20Object%20Reference) (OtherActor :type Actor%20Object%20Reference) (OtherComp :type Primitive%20Component%20Object%20Reference) (OtherBodyIndex :type Integer) (bFromSweep :type Boolean) (SweepResult :type Hit%20Result%20Structure%20%28by%20ref%29))
  (bind _returnvalue (Transformation|GetWorldLocation OtherComp))
  (bind _mesh (Variables|Character|GetMesh))
  (bind _closestworldposition (Class|SkeletalMeshComponent|GetClosestPointonPhysicsAsset _mesh _returnvalue))
  ;[0.15 0.15 0.15 0.5] 피격
  (bind _asbp_third_person_character (Utilities|Casting|CastToBP_ThirdPersonCharacter OtherActor)
    (:then
      (if (== OtherComp (Variables|/Game/ThirdPerson/Blueprints/BP_ThirdPersonCharacter.BP_ThirdPersonCharacter_C|GetItem _asbp_third_person_character))
        (if (or (Variables|/Game/ThirdPerson/Anim/ABP_Basic.ABP_Basic_C|GetAttackMode (Variables|/Game/ThirdPerson/Blueprints/BP_ThirdPersonCharacter.BP_ThirdPersonCharacter_C|GetAs%20ABP%20Basic _asbp_third_person_character)) (Variables|/Game/ThirdPerson/Anim/ABP_Basic.ABP_Basic_C|GetAttackMode2 (Variables|/Game/ThirdPerson/Blueprints/BP_ThirdPersonCharacter.BP_ThirdPersonCharacter_C|GetAs%20ABP%20Basic _asbp_third_person_character)))
          (Default|BloodCalculation _asbp_third_person_character)
          (Variables|/Game/Zombie/Anim_Zombie/ABP_Zombiegirl.ABP_Zombiegirl_C|SetHitMode (Variables|Default|GetAs%20ABP%20Zombiegirl) true)
          (Variables|Default|SetHP (- (Variables|Default|GetHP) (.AttackPower_Base (Utilities|Struct|BreakBat_Base (Variables|/Game/ThirdPerson/Blueprints/BP_ThirdPersonCharacter.BP_ThirdPersonCharacter_C|GetCurrent%20Row _asbp_third_person_character)))))
          (Default|Detect (Variables|Default|GetAs%20BP%20Zombiegirl%20Ctrl))
          (Variables|/Game/ThirdPerson/Blueprints/BP_ThirdPersonCharacter.BP_ThirdPersonCharacter_C|SetDurability _asbp_third_person_character (- (Variables|/Game/ThirdPerson/Blueprints/BP_ThirdPersonCharacter.BP_ThirdPersonCharacter_C|GetDurability _asbp_third_person_character) (.DurabilityDecrease_OnAttack (Utilities|Struct|BreakBat_Base (Variables|/Game/ThirdPerson/Blueprints/BP_ThirdPersonCharacter.BP_ThirdPersonCharacter_C|GetCurrent%20Row _asbp_third_person_character)))))
          (Audio|SpawnSoundatLocation (.HitSound (Utilities|Struct|BreakBat_Base (Variables|/Game/ThirdPerson/Blueprints/BP_ThirdPersonCharacter.BP_ThirdPersonCharacter_C|GetCurrent%20Row _asbp_third_person_character))) (Transformation|GetActorLocation) "0, 0, 0" 1.0 1.0 0.0 0 0)
          (Niagara|SpawnSystematLocation (.HitEffect (Utilities|Struct|BreakBat_Base (Variables|/Game/ThirdPerson/Blueprints/BP_ThirdPersonCharacter.BP_ThirdPersonCharacter_C|GetCurrent%20Row _asbp_third_person_character))) _closestworldposition (Math|Rotator|FindLookatRotation _returnvalue _closestworldposition))
          (if (.CanKnockdownZombie (Utilities|Struct|BreakBat_Base (Variables|/Game/ThirdPerson/Blueprints/BP_ThirdPersonCharacter.BP_ThirdPersonCharacter_C|GetCurrent%20Row _asbp_third_person_character)))
            (Variables|/Game/Zombie/Anim_Zombie/ABP_Zombiegirl.ABP_Zombiegirl_C|SetKnockDown (Variables|Default|GetAs%20ABP%20Zombiegirl) true))
          (elif (Variables|/Game/ThirdPerson/Anim/ABP_Basic.ABP_Basic_C|GetDefenseMode (Variables|/Game/ThirdPerson/Blueprints/BP_ThirdPersonCharacter.BP_ThirdPersonCharacter_C|GetAs%20ABP%20Basic _asbp_third_person_character))
            (Variables|/Game/Zombie/Anim_Zombie/ABP_Zombiegirl.ABP_Zombiegirl_C|SetHitMode (Variables|Default|GetAs%20ABP%20Zombiegirl) true)
            (Default|Detect (Variables|Default|GetAs%20BP%20Zombiegirl%20Ctrl))
            (Variables|/Game/ThirdPerson/Blueprints/BP_ThirdPersonCharacter.BP_ThirdPersonCharacter_C|SetDurability _asbp_third_person_character (- (Variables|/Game/ThirdPerson/Blueprints/BP_ThirdPersonCharacter.BP_ThirdPersonCharacter_C|GetDurability _asbp_third_person_character) (.DurabilityDecrease_OnBlock (Utilities|Struct|BreakBat_Base (Variables|/Game/ThirdPerson/Blueprints/BP_ThirdPersonCharacter.BP_ThirdPersonCharacter_C|GetCurrent%20Row _asbp_third_person_character)))))))))
    (:CastFailed
      (bind _asbp_bat_shoot (Utilities|Casting|CastToBP_BatShoot OtherActor))
      (Variables|/Game/Zombie/Anim_Zombie/ABP_Zombiegirl.ABP_Zombiegirl_C|SetHitMode (Variables|Default|GetAs%20ABP%20Zombiegirl) true)
      (Variables|Default|SetHP (- (Variables|Default|GetHP) (Variables|/Game/Items/BP_BatShoot.BP_BatShoot_C|GetAttackPower _asbp_bat_shoot)))
      (Default|Detect (Variables|Default|GetAs%20BP%20Zombiegirl%20Ctrl))
      (Audio|SpawnSoundatLocation "/Game/Sound/Hit/Hit.Hit" (Transformation|GetActorLocation) "0, 0, 0" 1.0 1.0 0.0 0 0)
      (Niagara|SpawnSystematLocation "/Game/Items/Effect/NE_BloodyEffect.NE_BloodyEffect" (.ClosestWorldPosition (Class|SkeletalMeshComponent|GetClosestPointonPhysicsAsset (Variables|Character|GetMesh) (Transformation|GetActorLocation _asbp_bat_shoot))) (Math|Rotator|FindLookatRotation (Transformation|GetActorLocation _asbp_bat_shoot) (.ClosestWorldPosition (Class|SkeletalMeshComponent|GetClosestPointonPhysicsAsset (Variables|Character|GetMesh) (Transformation|GetActorLocation _asbp_bat_shoot))))))))

(event OnComponentBeginOverlap(Box)
  (params (OverlappedComponent :type Primitive%20Component%20Object%20Reference) (OtherActor :type Actor%20Object%20Reference) (OtherComp :type Primitive%20Component%20Object%20Reference) (OtherBodyIndex :type Integer) (bFromSweep :type Boolean) (SweepResult :type Hit%20Result%20Structure%20%28by%20ref%29))
  ;[0.15 0.15 0.15 0.5] Assassination
  (bind _asbp_third_person_character (Utilities|Casting|CastToBP_ThirdPersonCharacter OtherActor))
  (if (and (not (ScalableFloat|GetValueasBool (AI|GetBlackboard (Variables|Default|GetAs%20BP%20Zombiegirl%20Ctrl)) (Utilities|Name|MakeLiteralName "Detected"))) (not (== OtherComp (Variables|/Game/ThirdPerson/Blueprints/BP_ThirdPersonCharacter.BP_ThirdPersonCharacter_C|GetNoiseSoundEffect _asbp_third_person_character))))
    (if (not (Variables|Default|GetDied))
      (Variables|/Game/ThirdPerson/Blueprints/BP_ThirdPersonCharacter.BP_ThirdPersonCharacter_C|SetZombiegirl _asbp_third_person_character self)
      (Default|Kill (Variables|/Game/ThirdPerson/Blueprints/BP_ThirdPersonCharacter.BP_ThirdPersonCharacter_C|GetWBP_Inform _asbp_third_person_character) true)
      (Widget|SetVisibility (Variables|/Game/ThirdPerson/Blueprints/BP_ThirdPersonCharacter.BP_ThirdPersonCharacter_C|GetWBP_Inform _asbp_third_person_character) "HitTestInvisible")
      (Variables|/Game/ThirdPerson/Blueprints/BP_ThirdPersonCharacter.BP_ThirdPersonCharacter_C|SetCanAssassin _asbp_third_person_character true))))

(event OnComponentEndOverlap(Box)
  (params (OverlappedComponent :type Primitive%20Component%20Object%20Reference) (OtherActor :type Actor%20Object%20Reference) (OtherComp :type Primitive%20Component%20Object%20Reference) (OtherBodyIndex :type Integer))
  ;[0.15 0.15 0.15 0.5] Assassination
  (bind _asbp_third_person_character (Utilities|Casting|CastToBP_ThirdPersonCharacter OtherActor))
  (Widget|SetVisibility (Variables|/Game/ThirdPerson/Blueprints/BP_ThirdPersonCharacter.BP_ThirdPersonCharacter_C|GetWBP_Inform _asbp_third_person_character) "Hidden")
  (Variables|/Game/ThirdPerson/Blueprints/BP_ThirdPersonCharacter.BP_ThirdPersonCharacter_C|SetCanAssassin _asbp_third_person_character false))

(event Custom|Assassined
  ;[0.15 0.15 0.15 0.5] Assassination
  (if (not (Variables|Default|GetDied))
    (Variables|Default|SetDied true)
    (AI|Components|Blackboard|SetValueasBool (AI|GetBlackboard (Variables|Default|GetAs%20BP%20Zombiegirl%20Ctrl)) (Utilities|Name|MakeLiteralName "Detected") false)
    (Variables|/Game/Zombie/Anim_Zombie/ABP_Zombiegirl.ABP_Zombiegirl_C|SetAssassin (Variables|Default|GetAs%20ABP%20Zombiegirl) true)))

(event Custom|Die
  ;[0.15 0.15 0.15 0.5] Die
  (if (not (Variables|Default|GetDied))
    (Variables|Default|SetDied true)
    (AI|Components|Blackboard|SetValueasBool (AI|GetBlackboard (Variables|Default|GetAs%20BP%20Zombiegirl%20Ctrl)) (Utilities|Name|MakeLiteralName "Detected") false)
    (Rendering|SetVisibility (Variables|Default|GetHPText) false false)
    (Variables|/Game/Zombie/Anim_Zombie/ABP_Zombiegirl.ABP_Zombiegirl_C|SetDie (Variables|Default|GetAs%20ABP%20Zombiegirl) true)
    (Utilities|Time|ClearandInvalidateTimerbyHandle (Variables|Default|GetAudioHandler))
    (bind _audio (Variables|Default|GetAudio)
      (:then
        (Audio|Components|Audio|Stop _audio))
      (:else
        _))
    (Utilities|FlowControl|Delay 5.0)
    (Actor|DestroyActor)))

(event Custom|Assassin%20died
  ;[0.15 0.15 0.15 0.5] Assassination
  (Rendering|SetVisibility (Variables|Default|GetHPText) false false)
  (Utilities|FlowControl|Delay 5.0)
  (Actor|DestroyActor))

(event Custom|Sound
  ;[0.15 0.15 0.15 0.5] Begin
  (Utilities|FlowControl|Delay (Math|Random|RandomFloatinRange 0.0 3.0))
  (bind _returnvalue (Audio|SpawnSoundatLocation "/Game/Sound/Zombie/ZombieS.ZombieS" (Transformation|GetActorLocation) "0, 0, 0" 1.0 1.0 0.0 0 0))
  (Variables|Default|SetAudio _returnvalue))

(event EventBeginPlay
  ;[0.15 0.15 0.15 0.5] Begin
  (bind _asabp_zombiegirl (Utilities|Casting|CastToABP_Zombiegirl (Components|SkeletalMesh|GetAnimInstance (Variables|Character|GetMesh))))
  (Variables|Default|SetAs%20ABP%20Zombiegirl _asabp_zombiegirl)
  (bind _asbp_zombie_girl_ctrl (Utilities|Casting|CastToBP_ZombieGirlCtrl (Pawn|GetController)))
  (Variables|Default|SetAs%20BP%20Zombiegirl%20Ctrl _asbp_zombie_girl_ctrl)
  (CallFunction|Sound)
  (bind _returnvalue (Utilities|Time|SetTimerbyEvent (delegate Custom|Sound) 6.0 true))
  (Variables|Default|SetAudioHandler _returnvalue))

(event EventTick
  (params (DeltaSeconds :type Float%20%28single-precision%29))
  (bind _hptext (Variables|Default|GetHPText))
  (bind _hp (Variables|Default|GetHP))
  ;[0.15 0.15 0.15 0.5] Tick
  (Transformation|SetWorldRotation _hptext (Math|Rotator|FindLookatRotation (Transformation|GetWorldLocation _hptext) (Transformation|GetActorLocation (Game|GetPlayerCameraManager 0))) false false)
  (Rendering|Components|TextRender|SetText _hptext (Utilities|Text|ToText(Float) _hp "HalfToEven"))
  (if (not (> _hp 0.0))
    (CallFunction|Die)))

(fn ConstructionScript)