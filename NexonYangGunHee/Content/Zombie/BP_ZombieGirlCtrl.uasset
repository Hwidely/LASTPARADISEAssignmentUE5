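; BP_ZombieGirlCtrl is the AI controller for the zombie girl enemy, running its behavior tree and handling detection of the player.
; On BeginPlay it runs BT_ZombieGirl and caches the controlled zombie pawn.
; When perception updates for the player, or Detect is called directly, a living, not-yet-detected zombie plays a detection sound and sets Detected in both the blackboard and its animation Blueprint.
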(event OnTargetPerceptionUpdated(AIPerception)
  (params (Actor :type Actor%20Object%20Reference) (Stimulus :type AI%20Stimulus%20Structure))
  (bind _as_zombiegirl (Variables|Default|GetAs%20Zombiegirl))
  (if (== Actor (Game|GetPlayerCharacter 0))
    (if (not (or (ScalableFloat|GetValueasBool (AI|GetBlackboard 0) (Utilities|Name|MakeLiteralName "Detected")) (Variables|/Game/Zombie/BP_ZombieGirl.BP_ZombieGirl_C|GetDied _as_zombiegirl)))
      (Audio|SpawnSoundatLocation "/Game/Sound/Zombie/zombieDetect.zombieDetect" (Transformation|GetActorLocation _as_zombiegirl) "0, 0, 0" 1.0 1.0 0.0 0 0)
      (AI|Components|Blackboard|SetValueasBool (AI|GetBlackboard 0) (Utilities|Name|MakeLiteralName "Detected") true)
      (Variables|/Game/Zombie/Anim_Zombie/ABP_Zombiegirl.ABP_Zombiegirl_C|SetDetected (Variables|/Game/Zombie/BP_ZombieGirl.BP_ZombieGirl_C|GetAs%20ABP%20Zombiegirl (Variables|Default|GetAs%20Zombiegirl)) true))))

(event Custom|Detect
  (bind _as_zombiegirl (Variables|Default|GetAs%20Zombiegirl))
  (if (not (or (ScalableFloat|GetValueasBool (AI|GetBlackboard 0) (Utilities|Name|MakeLiteralName "Detected")) (Variables|/Game/Zombie/BP_ZombieGirl.BP_ZombieGirl_C|GetDied _as_zombiegirl)))
    (Audio|SpawnSoundatLocation "/Game/Sound/Zombie/zombieDetect.zombieDetect" (Transformation|GetActorLocation _as_zombiegirl) "0, 0, 0" 1.0 1.0 0.0 0 0)
    (AI|Components|Blackboard|SetValueasBool (AI|GetBlackboard 0) (Utilities|Name|MakeLiteralName "Detected") true)
    (Variables|/Game/Zombie/Anim_Zombie/ABP_Zombiegirl.ABP_Zombiegirl_C|SetDetected (Variables|/Game/Zombie/BP_ZombieGirl.BP_ZombieGirl_C|GetAs%20ABP%20Zombiegirl (Variables|Default|GetAs%20Zombiegirl)) true)))

(event EventBeginPlay
  (AI|RunBehaviorTree "/Game/Zombie/BT_ZombieGirl.BT_ZombieGirl")
  (bind _asbp_zombie_girl (Utilities|Casting|CastToBP_ZombieGirl (Pawn|GetControlledPawn)))
  (Variables|Default|SetAs%20Zombiegirl _asbp_zombie_girl))

(fn ConstructionScript)